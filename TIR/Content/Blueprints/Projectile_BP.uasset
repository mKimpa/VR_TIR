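; Projectile for a VR shooter that ricochets, scores on targets and destroys itself by its third hit.
; Sphere hits route through a tag check: Wall and Bullet play Ricochet, while other actors pass their first tag to VrGameMode as HitColor, trigger scoring and destroy the projectile.
; Ammo hits also refill and reload the VR pawn, updating a material parameter collection.
; A separate Hit event spawns a shockwave aligned to the impact normal.
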(event `self.Sphere.OnComponentHit`
  (params (HitComponent :type "PrimitiveComponent Object Reference") (OtherActor :type "Actor Object Reference") (OtherComp :type "PrimitiveComponent Object Reference") (NormalImpulse :type "Vector Structure") (Hit :type "HitResult Structure (by ref)"))
  (`/Engine/EditorBlueprintResources/StandardMacros.IsValid` OtherActor
    (:`Is Valid`
      (`|ExecutionSequence`
        (:`then_0`
          (`self.HitFunction` OtherActor))
        (:`then_1`
          (bind _output_get (set `self.HitCount` (+ (`self.HitCount`) 1)))
          (if (== _output_get 3)
            (`self.K2_DestroyActor`)
            (set `self.HitCount` 0)))))))

(event `self.ReceiveHit`
  (params (MyComp :type "PrimitiveComponent Object Reference") (Other :type "Actor Object Reference") (OtherComp :type "PrimitiveComponent Object Reference") (bSelfMoved :type Boolean) (HitLocation :type "Vector Structure") (HitNormal :type "Vector Structure") (NormalImpulse :type "Vector Structure") (Hit :type "HitResult Structure (by ref)"))
  (bind (_returnvalue_roll _returnvalue_pitch _returnvalue_yaw) (`KismetMathLibrary.BreakRotator` (`KismetMathLibrary.Conv_VectorToRotator` (`.ImpactNormal` (`GameplayStatics.BreakHitResult` Hit)))))
  ;[1 1 1] Hit Effect (Shockwave)
  (`/Engine/EditorBlueprintResources/StandardMacros.IsValid` Other
    (:`Is Valid`
      (`|SpawnActorFromClass` "/Game/Blueprints/ShockWave_BP.Shockwave_BP_C" (`KismetMathLibrary.MakeTransform` HitLocation (`KismetMathLibrary.MakeRotator` _returnvalue_roll (- _returnvalue_pitch 90.0) _returnvalue_yaw)) "Undefined" "OverrideRootScale" null null))))

(fn `HitFunction`
  (params (self2 :type "Actor Object Reference"))
  (bind _output (`|GetArrayItem` (`Actor.Tags` self2)))
  (if (`self.ActorHasTag` self2 "Wall")
    (`AudioComponent.Play` (`self.Ricochet`) 0.0 :!label _label)
    (elif (`self.ActorHasTag` self2 "Ammo")
      (bind _asvr_game_mode (cast `/Game/Blueprints/VrGameMode` (`GameplayStatics.GetGameMode`)))
      (set `/Game/Blueprints/VrGameMode.HitColor` _output _asvr_game_mode)
      (bind _asvr_pawn (cast `/Game/Blueprints/VR_Pawn` (`GameplayStatics.GetPlayerPawn` 0)))
      (bind _output_get (set `/Game/Blueprints/VR_Pawn.AmmoCount` 1.0 _asvr_pawn))
      (`self.K2_DestroyActor`)
      (`/Game/Blueprints/VrGameMode.ScoreDP_Event` _asvr_game_mode)
      (`KismetMaterialLibrary.SetScalarParameterValue` "/Game/Blueprints/Ammo.Ammo" "Ammo" _output_get)
      (`/Game/Blueprints/VR_Pawn.ReloadFunction` _asvr_pawn)
      (elif (`self.ActorHasTag` self2 "Bullet")
        (goto _label)
        (else
          (bind _asvr_game_mode_2 (cast `/Game/Blueprints/VrGameMode` (`GameplayStatics.GetGameMode`)))
          (set `/Game/Blueprints/VrGameMode.HitColor` _output _asvr_game_mode_2)
          (`self.K2_DestroyActor`)
          (`/Game/Blueprints/VrGameMode.ScoreDP_Event` _asvr_game_mode_2))))))

(fn `UserConstructionScript`)