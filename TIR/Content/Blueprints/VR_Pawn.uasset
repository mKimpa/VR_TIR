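; VR player pawn with a gun that fires projectiles, doubles as a widget pointer, and is aimed by look-axis rotation of the azimuth and gun.
; Shots drain ammo and a delayed Tick slowly refills it, both updating a material parameter collection.
; Menu input or Resume_Event toggles the streamed UI level and pause flag, gated by start/name-entry widget visibility.
; Trigger animation is left unwired.
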(event `InputAxis|FireAnim`
  (params (AxisValue :type "Float (single-precision)"))
  (bind _asvr_gun_anim_bp (cast `/Game/Gun/VrGun_AnimBP` (`SkeletalMeshComponent.GetAnimInstance` (`self.VrGun`)))))

(event `InputAction|Fire`
  (params (Key :type "Key Structure"))
  (bind _widgetinteraction (`self.WidgetInteraction`))
  (:`Pressed`
    (`WidgetInteractionComponent.ReleasePointerKey` _widgetinteraction "LeftMouseButton")
    (if (`self.Pause`)
      _
      (elif (>= (`self.AmmoCount`) 0.0)
        (`|SpawnActorFromClass` "/Game/Blueprints/Projectile_BP.Projectile_BP_C" (`SceneComponent.K2_GetComponentToWorld` (`self.Arrow`)) "Undefined" "OverrideRootScale" null null)
        (bind _output_get (set `self.AmmoCount` (- (`self.AmmoCount`) 0.05)))
        (`AudioComponent.Play` (`self._Shot`) 0.0)
        (`KismetMaterialLibrary.SetScalarParameterValue` "/Game/Blueprints/Ammo.Ammo" "Ammo" _output_get))))
  (:`Released`
    (`WidgetInteractionComponent.PressPointerKey` _widgetinteraction "LeftMouseButton")))

(event `self.ReceiveTick`
  (params (DeltaSeconds :type "Float (single-precision)"))
  (bind _ammocount (`self.AmmoCount`))
  (`KismetSystemLibrary.Delay` 10.0)
  (if (< _ammocount 20.0)
    (bind _output_get (set `self.AmmoCount` (+ _ammocount 0.05)))
    (`KismetMaterialLibrary.SetScalarParameterValue` "/Game/Blueprints/Ammo.Ammo" "Ammo" _output_get)))

(event `InputAction|Menu`
  (params (Key :type "Key Structure"))
  (:`Pressed`
    (bind _outactors (`GameplayStatics.GetAllActorsOfClass` "/Game/UI/3DStartUI.3DStartUI_C" :!label _label))
    (bind _outactors_2 (`GameplayStatics.GetAllActorsOfClass` "/Game/UI/3DEnterNameUI.3DEnterNameUI_C"))
    (if (`KismetArrayLibrary.Array_IsValidIndex` _outactors_2)
      (if (not (`SceneComponent.bVisible` (`self.GetComponentByClass` (`|GetArrayItem` _outactors_2) "/Script/UMG.WidgetComponent")))
        (if (not (`SceneComponent.bVisible` (`self.GetComponentByClass` (`|GetArrayItem` _outactors) "/Script/UMG.WidgetComponent"))) :!label _label_2
          (`/Engine/EditorBlueprintResources/StandardMacros.FlipFlop`
            (:`A`
              (`GameplayStatics.LoadStreamLevel` "UI" true)
              (set `self.Pause` true))
            (:`B`
              (`GameplayStatics.UnloadStreamLevel` "UI")
              (set `self.Pause` false)))))
      (else
        (goto _label_2)))))

(event `Resume_Event`
  (goto _label))

(event `InputAxis|HorizontalLook`
  (params (AxisValue :type "Float (single-precision)"))
  (`SceneComponent.K2_AddLocalRotation` (`self.Azimuth`) (`KismetMathLibrary.MakeRotator` 0.0 0.0 (* AxisValue (`GameplayStatics.GetWorldDeltaSeconds`) 100.0)) false false))

(event `InputAxis|VerticalLook`
  (params (AxisValue :type "Float (single-precision)"))
  (`SceneComponent.K2_AddLocalRotation` (`self.VrGun`) (`KismetMathLibrary.MakeRotator` (* AxisValue (`GameplayStatics.GetWorldDeltaSeconds`) -100.0)) false false))

(fn `ReloadFunction`
  (`AudioComponent.Play` (`self.Reload`) 0.0))

(fn `UserConstructionScript`)