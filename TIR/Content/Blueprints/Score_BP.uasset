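; Score board actor that shows the countdown timer and score for a VR game and ends the round when time runs out.
; Tick, gated by the VR_Pawn's Pause flag, uses a one-second Delay to decrement the timer.
; Once it drops below zero, it plays EndGame, pauses the pawn and streams in the CreateName level after a short delay.
; The SetScore event refreshes the score digits until time is up.
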(event `self.ReceiveBeginPlay`
  (`TextRenderComponent.K2_SetText` (`self.TimerDigits`) (`KismetTextLibrary.Conv_IntToText` (`self.Timer`))))

(event `self.ReceiveTick`
  (params (DeltaSeconds :type "Float (single-precision)"))
  (bind _timer (`self.Timer`))
  ;[1 1 1] Game pause
  (bind _outactors (`GameplayStatics.GetAllActorsOfClass` "/Game/Blueprints/VR_Pawn.VR_Pawn_C"))
  (bind _output (`|GetArrayItem` _outactors))
  (if (not (`/Game/Blueprints/VR_Pawn.Pause` _output))
    ;[0 0 0] Timer
    (if (not (`self.TimeIsUp`))
      (`KismetSystemLibrary.Delay` 1.0)
      (bind _result (`/Engine/EditorBlueprintResources/StandardMacros.DecrementInt` _timer)
        (:`  `
          (set `self.Timer` _result)
          (if (== _timer -1)
            (set `self.TimeIsUp` true)
            (`AudioComponent.Play` (`self.EndGame`) 0.0)
            (set `/Game/Blueprints/VR_Pawn.Pause` true _output)
            (`KismetSystemLibrary.Delay` 1.0)
            (`GameplayStatics.LoadStreamLevel` "CreateName" true)
            (else
              (`TextRenderComponent.K2_SetText` (`self.TimerDigits`) (`KismetTextLibrary.Conv_IntToText` (`self.Timer`))))))))))

(event `/Game/Blueprints/ScoreInt.SetScore`
  (if (not (`self.TimeIsUp`))
    (`TextRenderComponent.K2_SetText` (`self.ScoreDigits`) (`KismetTextLibrary.Conv_IntToText` (`self.Score Text`)))))

(fn `UserConstructionScript`)