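; Actor Blueprint that recolors the level's stationary point lights over time from a timeline color track.
; On BeginPlay it gathers Stationary PointLight actors into an array at their search index, so skipped lights leave empty slots.
; Tick calls Play on the timeline, whose updates apply the current color to every stored light.
; The random delay is unconnected, and the random color index has no effect.
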(event `self.ReceiveBeginPlay`
  (`self.SetLight`))

(event `self.ReceiveTick`
  (params (DeltaSeconds :type "Float (single-precision)"))
  (bind (_direction _light) (`Timeline|Timeline_0`)
    (:`Update`
      (set `self.DinColor` _light)
      (`self.SetColor`))))

(fn `SetColor`
  (set `self.ColorIndex` (`KismetMathLibrary.RandomIntegerInRange` 0 4))
  (for _array_element (`self.Light`)
    (`LightComponent.SetLightColor` (`PointLight.PointLightComponent` _array_element) (`self.DinColor`) true)))

(fn `SetLight`
  (bind _outactors (`GameplayStatics.GetAllActorsOfClass` "/Script/Engine.PointLight"))
  (for (_array_element _array_index) _outactors
    (if (`|EnumEquality` (`SceneComponent.Mobility` (`PointLight.PointLightComponent` _array_element)) "Stationary")
      (`KismetArrayLibrary.Array_Set` (`self.Light`) _array_index _array_element true))))

(fn `UserConstructionScript`)