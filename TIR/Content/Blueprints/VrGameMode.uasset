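; VR game mode that keeps the player's score and handles high-score data.
; ScoreDP_Event runs UpdateScore, where consecutive same-color hits add growing powers of two, color changes or "Ammo" reset the streak, and scoring hits refresh the first Score_BP's display.
; SaveScore's branch is fixed true, ignoring the existence check, so it appends name and score to the loaded "HS" save without writing it back.
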(event `self.ReceiveBeginPlay`)

(event `ScoreDP_Event`
  (`self.UpdateScore`))

(fn `SaveScore`
  (`GameplayStatics.DoesSaveGameExist` "HS")
  (if true
    (bind _returnvalue (`GameplayStatics.LoadGameFromSlot` "HS"))
    (bind _ashs_save_data (cast `/Game/UI/HS_SaveData` _returnvalue))
    (bind _output_get (set `self.HSSave` _ashs_save_data))
    (`KismetArrayLibrary.Array_Add` (`/Game/UI/HS_SaveData.PlayerNames` _output_get) (`self.PlayerName`))
    (`KismetArrayLibrary.Array_Add` (`/Game/UI/HS_SaveData.PlayerScores` _output_get) (`self.Score`))
    (else
      (bind _returnvalue_2 (`GameplayStatics.CreateSaveGameObject` "/Game/UI/HS_SaveData.HS_SaveData_C"))
      (bind _ashs_save_data_2 (cast `/Game/UI/HS_SaveData` _returnvalue_2))
      (bind _output_get_2 (set `self.HSSave` _ashs_save_data_2))
      (`GameplayStatics.SaveGameToSlot` _output_get_2 "HS"))))

(fn `UpdateScore`
  (if (== (`self.HitColor`) "Ammo")
    (set `self.HitSequenceWeight` 0)
    (else
      (if (== (`self.HitSequenceWeight`) 0)
        _
        (elif (not (== (`self.LastHitColor`) (`self.HitColor`)))
          (set `self.HitSequenceWeight` 0)))
      (bind _result (`/Engine/EditorBlueprintResources/StandardMacros.IncrementInt` (`self.HitSequenceWeight`))
        (:`  `
          (set `self.LastHitColor` (`self.HitColor`))
          (bind _output_get (set `self.Score` (+ (`KismetMathLibrary.FTrunc` (`KismetMathLibrary.MultiplyMultiply_FloatFloat` 2.0 (`KismetMathLibrary.Conv_IntToDouble` _result))) (`self.Score`))))
          (bind _outactors (`GameplayStatics.GetAllActorsOfClass` "/Game/Blueprints/Score_BP.Score_BP_C"))
          (bind _output (`|GetArrayItem` _outactors))
          (set `/Game/Blueprints/Score_BP.Score Text` _output_get _output)
          (message `/Game/Blueprints/ScoreInt.SetScore` _output))))))

(fn `UserConstructionScript`)