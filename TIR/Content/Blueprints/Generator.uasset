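; Generator actor that scatters child actors at random points inside a box volume and reports their count to the score display as balls left.
; The construction script runs SpawnActors, which sizes the box from Extent and adds SpawnCount child actor components within it.
; It then writes the count to the first Score_BP found and unconditionally raises SpawnCount by a fixed step.
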(event `self.ReceiveTick`
  (params (DeltaSeconds :type "Float (single-precision)")))

(fn `SpawnActors`
  (bind _extent (`self.Extent`))
  (bind _spawncount (`self.SpawnCount`))
  (`BoxComponent.SetBoxExtent` (`self.Box`) _extent true)
  (for _ (range 1 (+ _spawncount 1))
    (`AddComponent|NODE_AddChildActorComponent-1` :`RelativeTransform` (`KismetMathLibrary.MakeTransform` (`KismetMathLibrary.RandomPointInBoundingBox` (0.0 0.0 0.0) _extent))))
  (bind _output_get (set `self.Count` _spawncount))
  (bind _outactors (`GameplayStatics.GetAllActorsOfClass` "/Game/Blueprints/Score_BP.Score_BP_C"))
  (`TextRenderComponent.K2_SetText` (`/Game/Blueprints/Score_BP.BallsLeftDigits` (`|GetArrayItem` _outactors)) (`KismetTextLibrary.Conv_IntToText` _output_get))
  (if true
    (set `self.SpawnCount` (+ _spawncount 3))))

(fn `UserConstructionScript`
  (`self.SpawnActors`))