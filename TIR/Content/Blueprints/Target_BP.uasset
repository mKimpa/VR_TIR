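; Destructible target that scales up on spawn with a random launch impulse and a color-matched tag, with one color made rarer by a reroll.
; Projectile_BP hits apply radial damage, while hits at roughly 0.6 scale spawn Shockwave_BP.
; Fracture plays effects, decrements the Generator's count and opens a Tick gate.
; That gate shrinks the target toward destruction, updates Score_BP's balls-left text and triggers Generator spawning at zero.
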(event `self.ReceiveBeginPlay`
  (`self.ColorRandomiser`)
  (`PrimitiveComponent.AddImpulse` (`self.Destructible`) (* (`KismetMathLibrary.RandomUnitVector`) (`KismetMathLibrary.RandomIntegerInRange` 600 800)) "None" false)
  (bind (_direction _newtrack_0) (`Timeline|ScaleUp`)
    (:`Update`
      (`SceneComponent.SetWorldScale3D` (`self.Destructible`) _newtrack_0))))

(event `self.ReceiveTick`
  (params (DeltaSeconds :type "Float (single-precision)"))
  (`/Engine/EditorBlueprintResources/StandardMacros.Gate` true :!label _label
    (:`Exit`
      (`self.ScaleDawn`)
      (bind _outactors (`GameplayStatics.GetAllActorsOfClass` "/Game/Blueprints/Score_BP.Score_BP_C"))
      (`TextRenderComponent.K2_SetText` (`/Game/Blueprints/Score_BP.BallsLeftDigits` (`|GetArrayItem` _outactors)) (`KismetTextLibrary.Conv_IntToText` (stale `self.Destructible.OnComponentFracture` _output_get)))
      (if (== (stale `self.Destructible.OnComponentFracture` _output_get) 0)
        (`/Game/Blueprints/Generator.SpawnActors` (`|GetArrayItem` (stale `self.Destructible.OnComponentFracture` _outactors)))))))

(event `self.Destructible.OnComponentFracture`
  (params (HitPoint :type "Vector Structure (by ref)") (HitDirection :type "Vector Structure (by ref)"))
  (`AudioComponent.Play` (`self._ShockWave`) 0.0)
  (`AudioComponent.Play` (`self.DestructionCue`) 0.0)
  (bind _outactors (`GameplayStatics.GetAllActorsOfClass` "/Game/Blueprints/Generator.Generator_C"))
  (bind _output (`|GetArrayItem` _outactors))
  (bind _result (`/Engine/EditorBlueprintResources/StandardMacros.DecrementInt` (`/Game/Blueprints/Generator.Count` _output))
    (:`  `
      (bind _output_get (set `/Game/Blueprints/Generator.Count` _result _output))
      (`PrimitiveComponent.SetCollisionEnabled` (`self.Destructible`) "NoCollision")
      (goto _label :!via `Open`))))

(event `self.Destructible.OnComponentHit`
  (params (HitComponent :type "PrimitiveComponent Object Reference") (OtherActor :type "Actor Object Reference") (OtherComp :type "PrimitiveComponent Object Reference") (NormalImpulse :type "Vector Structure") (Hit :type "HitResult Structure (by ref)"))
  (bind _asprojectile_bp (cast `/Game/Blueprints/Projectile_BP` OtherActor))
  (`GameplayStatics.ApplyRadialDamage` :`BaseDamage` 1.0 :`Origin` (`.ImpactPoint` (`GameplayStatics.BreakHitResult` Hit)) :`DamageRadius` 10.0 :`DamageCauser` _asprojectile_bp :`InstigatedByController` null))

(event `self.ReceiveHit`
  (params (MyComp :type "PrimitiveComponent Object Reference") (Other :type "Actor Object Reference") (OtherComp :type "PrimitiveComponent Object Reference") (bSelfMoved :type Boolean) (HitLocation :type "Vector Structure") (HitNormal :type "Vector Structure") (NormalImpulse :type "Vector Structure") (Hit :type "HitResult Structure (by ref)"))
  (bind (_returnvalue_roll _returnvalue_pitch _returnvalue_yaw) (`KismetMathLibrary.BreakRotator` (`KismetMathLibrary.Conv_VectorToRotator` (`.ImpactNormal` (`GameplayStatics.BreakHitResult` Hit)))))
  ;[0.07812 0.07812 0.07812] Spawn Shockwave
  (`/Engine/EditorBlueprintResources/StandardMacros.IsValid` Other
    (:`Is Valid`
      (if (== (`SceneComponent.RelativeScale3D` (`self.Destructible`)) (0.6 0.6 0.6) :`ErrorTolerance` 0.1)
        (`|SpawnActorFromClass` "/Game/Blueprints/ShockWave_BP.Shockwave_BP_C" (`KismetMathLibrary.MakeTransform` HitLocation (`KismetMathLibrary.MakeRotator` _returnvalue_roll (- _returnvalue_pitch 90.0) _returnvalue_yaw)) "Undefined" "OverrideRootScale" null null)))))

(fn `ColorRandomiser`
  (bind _output_get (set `self.ColorIndex` (`KismetMathLibrary.RandomIntegerInRange` 0 5) :!label _label))
  (if (== _output_get 5)
    (if (`KismetMathLibrary.RandomBoolWithWeight` 0.5)
      _
      (else
        (goto _label))))
  (bind _returnvalue (`KismetMaterialLibrary.CreateDynamicMaterialInstance` "/Game/Materials/TargetAutomat.TargetAutomat"))
  (`PrimitiveComponent.SetMaterial` (`self.Destructible`) 0 _returnvalue)
  (`MaterialInstanceDynamic.SetVectorParameterValue` _returnvalue "Color" (`|GetArrayItem` (`self.Color`) (`self.ColorIndex`)))
  (`SceneComponent.SetWorldScale3D` (`self.Destructible`) (0.0 0.0 0.0))
  (set `self.Tags` (`|MakeArray` (`|GetArrayItem` (`self.ColorTag`) (`self.ColorIndex`)))))

(fn `ScaleDawn`
  (bind _destructible (`self.Destructible`))
  (bind _returnvalue (* (`SceneComponent.RelativeScale3D` _destructible) (`KismetMathLibrary.FInterpEaseInOut` 1.0 0.0 (`GameplayStatics.GetWorldDeltaSeconds`) 1.0)))
  (`SceneComponent.SetWorldScale3D` _destructible _returnvalue)
  (if (== _returnvalue (0.01 0.01 0.01))
    (`self.K2_DestroyActor`)))

(fn `UserConstructionScript`)